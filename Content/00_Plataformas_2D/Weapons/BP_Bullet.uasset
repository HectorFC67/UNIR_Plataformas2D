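; Projectile actor for the 2D platformer's weapons that flies forward at a set speed and plays a shot sound on spawn.
; Tick moves it with a swept SetActorLocation rather than a movement component, and a timer destroys it after a short lifetime.
; Overlapping a Pawn deals damage, while a Sphere hit handles other impacts; both spawn an explosion, play their own sound and destroy the bullet after a brief delay.
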(event OnComponentHit(Sphere)
  (params (HitComponent :type Primitive%20Component%20Object%20Reference) (OtherActor :type Actor%20Object%20Reference) (OtherComp :type Primitive%20Component%20Object%20Reference) (NormalImpulse :type Vector :default "0, 0, 0") (Hit :type Hit%20Result%20Structure%20%28by%20ref%29))
  (Development|PrintString "Bullet Collision")
  (Effects|SpawnEmitteratLocation "/Game/StarterContent/Particles/P_Explosion.P_Explosion" (.location Hit))
  (Audio|PlaySound2D "/Game/Audio/GolpePared.GolpePared" 1.0 1.0 0.0 0 0)
  (Utilities|FlowControl|Delay 0.1)
  (Actor|DestroyActor))

(event Custom|DestroyBullet
  (Actor|DestroyActor))

(event EventBeginPlay
  (Audio|PlaySound2D "/Game/Audio/Disparo.Disparo" 1.0 1.0 0.0 0 0)
  (Utilities|Time|SetTimerbyEvent (delegate Custom|DestroyBullet) 3.0))

(event Collision|EventActorBeginOverlap
  (params (OtherActor :type Actor%20Object%20Reference))
  (bind _aspawn (Utilities|Casting|CastToPawn OtherActor))
  (Effects|SpawnEmitteratLocation "/Game/StarterContent/Particles/P_Explosion.P_Explosion" (Transformation|GetActorLocation))
  (Audio|PlaySound2D "/Game/Audio/ImpactoBala.ImpactoBala" 1.0 1.0 0.0 0 0)
  (Utilities|FlowControl|Delay 0.1)
  (Game|Damage|ApplyDamage _aspawn 1.0 0 self)
  (Actor|DestroyActor))

(event EventTick
  (params (DeltaSeconds :type Float%20%28single-precision%29))
  (Transformation|SetActorLocation (+ (Transformation|GetActorLocation) (* (* (Variables|Default|Getspeed) DeltaSeconds) (Transformation|GetActorForwardVector))) true false))

(fn ConstructionScript)